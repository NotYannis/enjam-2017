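; Tutorial fish pawn for the DonNavigation samples that follows spline patrol routes and carries a blackboard-driven Hunt state.
; When WaitForTrigger is set, BeginPlay bypasses the parent's startup and builds patrol goals from the PatrolActor spline.
; StartMoving fires CallTriggerActor, while StopMoving clears HearShot and Hunt and loads the SecondPatrol spline as the new route.
; Tick resets TriggerAll while no shot is heard and prints the Hunt flag for debugging.
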(event `self.ReceiveBeginPlay`
  (bind _patrolactor (`self.patrolActor`))
  (bind _returnvalue (`self.GetComponentByClass` _patrolactor "/Script/Engine.SplineComponent"))
  (if (`self.waitForTrigger`)
    (bind _asfloating_pawn_movement (cast `FloatingPawnMovement` (`self.MovementComponent`)))
    (set `self.floatingMovement` _asfloating_pawn_movement)
    (`/Engine/EditorBlueprintResources/StandardMacros.IsValid` _patrolactor
      (:`Is Valid`
        (`/Engine/EditorBlueprintResources/StandardMacros.IsValid` _returnvalue
          (:`Is Valid`
            (bind _output_get (set `self.patrolSpline` _returnvalue))
            (for _index (range (+ (`SplineComponent.GetNumberOfSplinePoints` _output_get) 1))
              (`KismetArrayLibrary.Array_Add` (`self.patrolGoals`) (`SplineComponent.GetLocationAtSplinePoint` (`self.patrolSpline`) _index "World"))))
          (:`Is Not Valid`
            (`KismetSystemLibrary.PrintString` "Need spline component on actor !" true true (struct :`R` 1.0 :`G` 0.017204 :`A` 1.0) :!label _label))))
      (:`Is Not Valid`
        (goto _label)))
    (else
      (`parent.ReceiveBeginPlay`))))

(event `StartMoving`
  (`/Game/EpicContent/DemoRoom/BluePrint/BPInterface_Button.CallTriggerActor`))

(event `StopMoving`
  (bind _secondpatrol (`self.secondPatrol`))
  (bind _returnvalue (`self.GetComponentByClass` _secondpatrol "/Script/Engine.SplineComponent"))
  (set `self.hearShot` false)
  (`BlackboardComponent.SetValueAsBool` (`AIBlueprintHelperLibrary.GetBlackboard` self) (`KismetStringLibrary.Conv_StringToName` "Hunt") false)
  (`/Engine/EditorBlueprintResources/StandardMacros.IsValid` _secondpatrol
    (:`Is Valid`
      (`/Engine/EditorBlueprintResources/StandardMacros.IsValid` _returnvalue
        (:`Is Valid`
          (bind _output_get (set `self.patrolSpline` _returnvalue))
          (`KismetArrayLibrary.Array_Clear` (`self.patrolGoals`))
          (for _index (range (+ (`SplineComponent.GetNumberOfSplinePoints` _output_get) 1))
            (`KismetArrayLibrary.Array_Add` (`self.patrolGoals`) (`SplineComponent.GetLocationAtSplinePoint` (`self.patrolSpline`) _index "World"))))
        (:`Is Not Valid`
          (`KismetSystemLibrary.PrintString` "Need spline component on actor !" true true (struct :`R` 1.0 :`G` 0.017204 :`A` 1.0) :!label _label_2))))
    (:`Is Not Valid`
      (goto _label_2))))

(event `self.ReceiveActorBeginOverlap`
  (params (OtherActor :type "Actor Object Reference"))
  (`parent.ReceiveActorBeginOverlap` OtherActor))

(event `self.ReceiveTick`
  (params (DeltaSeconds :type "Float (single-precision)"))
  (if (not (`self.hearShot`))
    (set `self.triggerAll` false))
  (`parent.ReceiveTick` DeltaSeconds)
  (`KismetSystemLibrary.PrintString` (`KismetStringLibrary.Conv_BoolToString` (`BlackboardComponent.GetValueAsBool` (`AIBlueprintHelperLibrary.GetBlackboard` self) (`KismetStringLibrary.Conv_StringToName` "Hunt")))))

(fn `UserConstructionScript`
  (`parent.UserConstructionScript`))